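; AI-controlled actor BP_mamo01 that destroys itself on its first capsule hit and awards score.
; From BeginPlay, a looping Delay event calls StopMovement on its AI controller every half second.
; The hit, guarded by DoOnce, sends SindaMessage to whatever actor it touched before destroying itself.
; Any destruction, including that one, sends ScrPlusMessage to the player pawn to add 500 points.
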(event `self.ReceiveBeginPlay`
  (`self.stpMov`))

(event `stpMov`
  (`KismetSystemLibrary.Delay` 0.5 :!label _label)
  (`Controller.StopMovement` (`AIBlueprintHelperLibrary.GetAIController` self))
  (goto _label))

(event `self.CapsuleComponent.OnComponentHit`
  (params (HitComponent :type "PrimitiveComponent Object Reference") (OtherActor :type "Actor Object Reference") (OtherComp :type "PrimitiveComponent Object Reference") (NormalImpulse :type "Vector Structure") (Hit :type "HitResult Structure (by ref)"))
  (`/Engine/EditorBlueprintResources/StandardMacros.DoOnce` false
    (:`Completed`
      (message `/Game/BP/BPI_CHi.sinda` OtherActor)
      (`self.K2_DestroyActor`))))

(event `self.ReceiveDestroyed`
  (message `/Game/BP/BPI_CHi.scrPlus` (`GameplayStatics.GetPlayerPawn` 0) 500))

(fn `UserConstructionScript`)